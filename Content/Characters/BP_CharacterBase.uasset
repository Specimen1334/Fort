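; Base player character for a networked cursor-aimed shooter with weapon inventory, grenades, melee, dashing and experience points.
; Enhanced Input drives actions, with weapon, melee and grenade logic routed through server and multicast events.
; Mouse aim intersects the cursor ray with a muzzle-height plane, while dashes lerp invincibly to the furthest valid capsule-tested spot on timer-refilled charges.
; Death plays a montage, then restores health at the initial transform.
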(event `self.ReceiveBeginPlay`
  (bind _returnvalue (`GameplayStatics.GetPlayerController` 0))
  (bind _returnvalue_2 (pcsubsystem `EnhancedInputLocalPlayerSubsystem` _returnvalue))
  ;[1 1 1] Begin Play
  (`|ExecutionSequence`
    (:`then_0`
      ;[1 1 1] Enhanced Input
      (if (`Controller.IsLocalPlayerController` _returnvalue)
        (`EnhancedInputSubsystemInterface.AddMappingContext` _returnvalue_2 "/Game/TSS_Game/Blueprints/EnhancedInput/InputMapping_KeyboardMouse.InputMapping_KeyboardMouse" 1 (struct))
        (`EnhancedInputSubsystemInterface.AddMappingContext` _returnvalue_2 "/Game/TSS_Game/Blueprints/EnhancedInput/InputMapping_Gamepad.InputMapping_Gamepad" 0 (struct))))
    (:`then_1`
      (bind _asbp_game_instance_with_settings (cast `/Game/TSS_Game/Blueprints/GameInstanceSettings/BP_GameInstanceWithSettings` (`GameplayStatics.GetGameInstance`)))
      (`/Game/TSS_Game/Blueprints/GameInstanceSettings/BP_GameInstanceWithSettings.LoadSettings` _asbp_game_instance_with_settings)
      (set `self.MouseRotationEnabled` (`/Game/TSS_Game/Blueprints/GameInstanceSettings/BP_GameInstanceWithSettings.SettingsMouseRotation` _asbp_game_instance_with_settings))
      (set `self.TransformForRespawn` (`self.GetTransform`))
      (set `self.Springarm_DefaultDistance` (`SpringArmComponent.TargetArmLength` (`self.SpringArm`)))
      (if (`self.UseStartingWeapon`)
        (`self.SpawnWeapon` (`self.DefaultWeaponClass`))))))

(event `ServerReloadEvent`
  (bind _equippedweapon (`self.EquippedWeapon`))
  ;[1 1 1] Weapon
  (`/Engine/EditorBlueprintResources/StandardMacros.IsValid` _equippedweapon
    (:`Is Valid`
      (`/Game/TSS_Game/Blueprints/Weapons/Base/BP_WeaponBase.Reload` _equippedweapon))))

(event `EnhancedInput|/Game/TSS_Game/Blueprints/EnhancedInput/InputAction_Reload`
  (params (ActionValue :type Boolean) (ElapsedSeconds :type "Float (double-precision)") (TriggeredSeconds :type "Float (double-precision)") (InputAction :type "InputAction Object Reference" :default "/Game/TSS_Game/Blueprints/EnhancedInput/InputAction_Reload.InputAction_Reload"))
  ;[1 1 1] Weapon
  (:`Triggered`
    (`self.ServerReloadEvent`)))

(event `WeaponSwitch`
  ;[1 1 1] Weapon
  (if (> (`KismetArrayLibrary.Array_Length` (`self.UT_Inventory`)) 0)
    (if (not (`self.isSwitchingWeapons`))
      (set `self.isSwitchingWeapons` true)
      (`self.EquipWeapon` (`self.CycleTroughInventory`))
      (`self.MulticastEquipMontage`))))

(event `MulticastEquipMontage`
  ;[1 1 1] Weapon
  (bind _returnvalue (`AnimInstance.Montage_Play` (`SkeletalMeshComponent.GetAnimInstance` (`self.Mesh`)) "/Game/TSS_Game/Character/AnimStarterPack/Equip_Rifle_Standing_Montage.Equip_Rifle_Standing_Montage" 2.0 "Duration" 0.0 true))
  (`KismetSystemLibrary.Delay` _returnvalue)
  (set `self.isSwitchingWeapons` false))

(event `EnhancedInput|/Game/TSS_Game/Blueprints/EnhancedInput/InputAction_WeaponSwitch`
  (params (ActionValue :type Boolean) (ElapsedSeconds :type "Float (double-precision)") (TriggeredSeconds :type "Float (double-precision)") (InputAction :type "InputAction Object Reference" :default "/Game/TSS_Game/Blueprints/EnhancedInput/InputAction_WeaponSwitch.InputAction_WeaponSwitch"))
  ;[1 1 1] Weapon
  (:`Triggered`
    (`self.WeaponSwitch`)))

(event `MulticastRotation`
  (bind _owningplayercontroller (`self.OwningPlayerController`))
  (bind (_worldlocation _worlddirection) (`PlayerController.DeprojectMousePositionToWorld` (`self.OwningPlayerController`)))
  (bind (_worldlocation_2 _worlddirection_2) (`PlayerController.DeprojectMousePositionToWorld` (`self.OwningPlayerController`)))
  ;[1 1 1] WASD
  (bind (_outhit _returnvalue) (`KismetSystemLibrary.LineTraceSingle` _worldlocation_2 (+ _worlddirection_2 (* _worlddirection_2 100000.0)) "TraceTypeQuery1" :!label _label))
  (if _returnvalue
    (if (`self.IsLocallyControlled`)
      (bind (_returnvalue_roll _returnvalue_pitch) (`KismetMathLibrary.BreakRotator` (`KismetMathLibrary.FindLookAtRotation` (`SceneComponent.K2_GetComponentLocation` (`self.CapsuleComponent`)) (`.Location` (`GameplayStatics.BreakHitResult` _outhit)))))
      (set `self.Rotation` (`KismetMathLibrary.NegateRotator` (`KismetMathLibrary.MakeRotator` _returnvalue_pitch)))
      (`/Engine/EditorBlueprintResources/StandardMacros.IsValid` _owningplayercontroller
        (:`Is Valid`
          (`Controller.SetControlRotation` _owningplayercontroller (`KismetMathLibrary.MakeRotator` 0.0 0.0 (.yaw (`KismetMathLibrary.RInterpTo` (`self.K2_GetActorRotation`) (`KismetMathLibrary.FindLookAtRotation` (`self.K2_GetActorLocation`) (`.Intersection` (`KismetMathLibrary.LinePlaneIntersection_OriginNormal` _worldlocation (+ _worldlocation (* _worlddirection 10000)) (`SceneComponent.K2_GetComponentLocation` (`self.BulletSpawnLocation`)) (0.0 0.0 1.0)))) (`GameplayStatics.GetWorldDeltaSeconds`) 20.0)))))))))

(event `self.ReceiveTick`
  (params (DeltaSeconds :type "Float (single-precision)"))
  ;[1 1 1] WASD
  (set `CharacterMovementComponent.MaxWalkSpeed` (`self.PlayerSpeed`) (`self.CharacterMovement`))
  (if (`self.MouseRotationEnabled`)
    (if (not (`self.IsDead`))
      (`/Engine/EditorBlueprintResources/StandardMacros.IsValid` (`self.OwningPlayerController`)
        (:`Is Valid`
          (`/Engine/EditorBlueprintResources/ActorMacros.Switch Has Authority`
            (:`Authority`
              (goto _label))
            (:`Remote`
              (`self.MulticastRotation`))))))))

(event `EnhancedInput|/Game/TSS_Game/Blueprints/EnhancedInput/InputAction_Aim`
  (params (ActionValue :type Boolean) (ElapsedSeconds :type "Float (double-precision)") (TriggeredSeconds :type "Float (double-precision)") (InputAction :type "InputAction Object Reference" :default "/Game/TSS_Game/Blueprints/EnhancedInput/InputAction_Aim.InputAction_Aim"))
  ;[1 1 1] Camera Zoom
  (:`Started`
    (bind (_direction _alpha) (`Timeline|CameraZoomTL` :!label _label_2)
      (:`Update`
        (set `SpringArmComponent.TargetArmLength` (`KismetMathLibrary.Lerp` (`self.Springarm_DefaultDistance`) (* (`self.Springarm_DefaultDistance`) 1.2) _alpha) (`self.SpringArm`)))))
  (:`Completed`
    (goto _label_2 :!via `Reverse`)))

(event `InputAxis|MoveForward`
  (params (AxisValue :type "Float (single-precision)"))
  ;[1 1 1] WASD
  (`self.AddMovementInput` (`KismetMathLibrary.GetForwardVector` (struct)) AxisValue))

(event `InputAxis|MoveRight`
  (params (AxisValue :type "Float (single-precision)"))
  ;[1 1 1] WASD
  (`self.AddMovementInput` (`KismetMathLibrary.GetRightVector` (struct)) AxisValue))

(event `InputAxis|LookUp`
  (params (AxisValue :type "Float (single-precision)"))
  (bind _owningplayercontroller (`self.OwningPlayerController`))
  ;[1 1 1] WASD
  (bind _returnvalue (`KismetMathLibrary.MakeVector` AxisValue (stale `InputAxis|LookRight` AxisValue)))
  (if (> (`KismetMathLibrary.VSize` _returnvalue) 0.25) :!label _label_3
    (`/Engine/EditorBlueprintResources/StandardMacros.IsValid` _owningplayercontroller
      (:`Is Valid`
        (`Controller.SetControlRotation` _owningplayercontroller (`KismetMathLibrary.Conv_VectorToRotator` _returnvalue))))))

(event `InputAxis|LookRight`
  (params (AxisValue :type "Float (single-precision)"))
  ;[1 1 1] WASD
  (goto _label_3))

(event `DashBegin`
  ;[1 1 1] WASD
  (`self.CanDash`
    (:`Yes`
      (set `self.IsDashing` true)
      (set `self.IsInvincible` true)
      (`/Engine/EditorBlueprintResources/StandardMacros.DecrementInt` (`self.AvailableDashCount`)
        (:`  `
          (`self.DashCooldownBegin`)
          (`|PlayMontage` (`self.Mesh`) null (/ 0.8 (`self.DashDuration`) 2.0)
            (:`then`
              (`self.MoveOverTime` (`self.GetFurthestValidLocationAlongRoute` (`self.K2_GetActorLocation`) (`self.Calculate Dash Target Location`))))))))))

(event `MoveOverTime`
  (params (Location :type "Vector Structure"))
  ;[1 1 1] WASD
  (bind _output_get (set `self.DashStartLocation` (`self.K2_GetActorLocation`)))
  (`self.K2_SetActorRotation` (`KismetMathLibrary.FindLookAtRotation` _output_get Location))
  (`TimelineComponent.SetPlayRate` (`self.DashTimeline`) (/ 1.0 (`self.DashDuration`)))
  (bind (_direction _alphalocation) (`Timeline|DashTimeline` :!via `PlayFromStart`)
    (:`Update`
      (`self.K2_SetActorLocation` (`KismetMathLibrary.VLerp` (`self.DashStartLocation`) Location _alphalocation)))
    (:`Finished`
      (set `self.IsDashing` false)
      (set `self.IsInvincible` false))))

(event `DashCooldownBegin`
  ;[1 1 1] WASD
  (`KismetSystemLibrary.K2_SetTimerDelegate` (delegate `ResetDashCount`) (`self.DashCooldown`)))

(event `ResetDashCount`
  ;[1 1 1] WASD
  (set `self.AvailableDashCount` (+ (`self.AvailableDashCount`) 1)))

(event `EnhancedInput|/Game/TSS_Game/Blueprints/EnhancedInput/InputAction_Fire`
  (params (ActionValue :type Boolean) (ElapsedSeconds :type "Float (double-precision)") (TriggeredSeconds :type "Float (double-precision)") (InputAction :type "InputAction Object Reference" :default "/Game/TSS_Game/Blueprints/EnhancedInput/InputAction_Fire.InputAction_Fire"))
  ;[1 1 1] Weapon
  (:`Started`
    (`self.ServerFireEvent`)))

(event `ServerFireEvent`
  (bind _equippedweapon (`self.EquippedWeapon`))
  ;[1 1 1] Weapon
  (if (not (`self.isSwitchingWeapons`))
    (`/Engine/EditorBlueprintResources/StandardMacros.IsValid` _equippedweapon
      (:`Is Valid`
        (`/Game/TSS_Game/Blueprints/Weapons/Base/BP_WeaponBase.Fire` _equippedweapon)))))

(event `ServerStopFire`
  (bind _equippedweapon (`self.EquippedWeapon`))
  ;[1 1 1] Weapon
  (`/Engine/EditorBlueprintResources/StandardMacros.IsValid` _equippedweapon
    (:`Is Valid`
      (`/Game/TSS_Game/Blueprints/Weapons/Base/BP_WeaponBase.StopWeaponFire` _equippedweapon))))

(event `EnhancedInput|/Game/TSS_Game/Blueprints/EnhancedInput/InputAction_Dash`
  (params (ActionValue :type Boolean) (ElapsedSeconds :type "Float (double-precision)") (TriggeredSeconds :type "Float (double-precision)") (InputAction :type "InputAction Object Reference" :default "/Game/TSS_Game/Blueprints/EnhancedInput/InputAction_Dash.InputAction_Dash"))
  ;[1 1 1] Jump & Crouch
  (:`Triggered`
    (`self.DashBegin`)))

(event `EnhancedInput|/Game/TSS_Game/Blueprints/EnhancedInput/InputAction_Crouch`
  (params (ActionValue :type Boolean) (ElapsedSeconds :type "Float (double-precision)") (TriggeredSeconds :type "Float (double-precision)") (InputAction :type "InputAction Object Reference" :default "/Game/TSS_Game/Blueprints/EnhancedInput/InputAction_Crouch.InputAction_Crouch"))
  ;[1 1 1] Jump & Crouch
  (:`Started`
    (`self.Crouch`))
  (:`Completed`
    (`self.UnCrouch`)))

(event `self.ReceiveAnyDamage`
  (params (Damage :type "Float (single-precision)") (DamageType :type "DamageType Object Reference") (InstigatedBy :type "Controller Object Reference") (DamageCauser :type "Actor Object Reference"))
  ;[1 1 1] Health
  (if (not (`self.IsInvincible`))
    (bind _output_get (set `self.HealthCurrent` (`KismetMathLibrary.FClamp` (- (`self.HealthCurrent`) Damage) 0.0 (`self.HealthMax`))))
    (if (<= _output_get 0.0)
      (`/Engine/EditorBlueprintResources/StandardMacros.DoOnce` false :!label _label_4
        (:`Completed`
          (set `self.IsDead` true)
          (`self.PlayerDied`)
          (`self.Multicast_DeathMontage`))))))

(event `Multicast_DeathMontage`
  ;[1 1 1] Health
  (`AnimInstance.Montage_Play` (`SkeletalMeshComponent.GetAnimInstance` (`self.Mesh`)) "/Game/TSS_Game/Character/AnimStarterPack/Death_2_Montage.Death_2_Montage" 1.0 "MontageLength" 0.0 true)
  (`self.UnCrouch`))

(event `PlayerDied`
  ;[1 1 1] Health
  (`self.DisableInput` (`self.OwningPlayerController`))
  (`self.ServerStopFire`)
  (`KismetSystemLibrary.RetriggerableDelay` 1.9) ; Duration of the death montage
  (`self.EnableInput` (`self.OwningPlayerController`))
  (`self.MulticastTeleport` (`self.TransformForRespawn`)))

(event `ServerTeleport`
  (params (NewTransform :type "Transform Structure (by ref)"))
  ;[1 1 1] Health
  (`self.K2_SetActorTransform` NewTransform false true)
  (set `self.HealthCurrent` (`self.HealthMax`))
  (set `self.IsDead` false)
  (goto _label_4 :!via `Reset`))

(event `MulticastTeleport`
  (params (NewTransform :type "Transform Structure (by ref)"))
  ;[1 1 1] Health
  (`self.ServerTeleport` NewTransform))

(event `Interaction`
  (params (Start :type "Vector Structure") (End :type "Vector Structure") (CharacterReference :type "/Game/Characters/BP_CharacterBase Object Reference"))
  ;[1 1 1] Interact
  (`self.InteractMulti` Start End CharacterReference))

(event `InteractMulti`
  (params (Start :type "Vector Structure") (End :type "Vector Structure") (CharacterReference :type "/Game/Characters/BP_CharacterBase Object Reference"))
  ;[1 1 1] Interact
  (bind (_outhit _returnvalue) (`KismetSystemLibrary.SphereTraceSingleForObjects` Start End 52.0 (`|MakeArray` "ObjectTypeQuery9" :!type "EObjectTypeQuery Enum") false (`self.UT_Inventory`)))
  (if _returnvalue
    (message `/Game/TSS_Game/Blueprints/System/BPI_Interactive.InteractWithWeapon` (`.HitActor` (`GameplayStatics.BreakHitResult` _outhit)) CharacterReference)))

(event `EnhancedInput|/Game/TSS_Game/Blueprints/EnhancedInput/InputAction_Interact`
  (params (ActionValue :type Boolean) (ElapsedSeconds :type "Float (double-precision)") (TriggeredSeconds :type "Float (double-precision)") (InputAction :type "InputAction Object Reference" :default "/Game/TSS_Game/Blueprints/EnhancedInput/InputAction_Interact.InputAction_Interact"))
  (bind _returnvalue (`self.K2_GetActorLocation`))
  ;[1 1 1] Interact
  (:`Triggered`
    (`self.Interaction` (+ _returnvalue (0.0 0.0 50.0)) (- _returnvalue (0.0 0.0 50.0)) self)))

(event `self.ReceiveDestroyed`
  (bind _ut_inventory (`self.UT_Inventory`))
  ;[1 1 1] When a player disconnects from the server, get rid of its weapons
  (if (> (`KismetArrayLibrary.Array_Length` _ut_inventory) 0)
    (for _array_element _ut_inventory
      (`/Engine/EditorBlueprintResources/StandardMacros.IsValid` _array_element
        (:`Is Valid`
          (`self.K2_DestroyActor` _array_element))))))

(event `Server_Melee`
  ;[1 1 1] Melee
  (`self.Multi_Melee`))

(event `Multi_Melee`
  (bind _returnvalue (`SceneComponent.K2_GetComponentLocation` (`self.CapsuleComponent`)))
  ;[1 1 1] Melee
  (if (not (`self.IsMeleeAttacking`))
    (set `self.IsMeleeAttacking` true)
    (`AnimInstance.Montage_Play` (`SkeletalMeshComponent.GetAnimInstance` (`self.Mesh`)) "/Game/TSS_Game/Character/AnimStarterPack/Fire_Rifle_Ironsights_Montage.Fire_Rifle_Ironsights_Montage" 1.0 "Duration" 0.0 true)
    (`|ExecutionSequence`
      (:`then_0`
        (bind (_outhit _returnvalue_2) (`KismetSystemLibrary.LineTraceSingle` (+ _returnvalue (0.0 0.0 45.0)) (+ _returnvalue (* (`KismetMathLibrary.GetForwardVector` (`self.K2_GetActorRotation`)) 100.0)) "TraceTypeQuery1" false (`self.UT_Inventory`)))
        (if _returnvalue_2
          (bind (_bblockinghit _binitialoverlap _time _distance _location _impactpoint _normal _impactnormal _physmat _hitactor) (`GameplayStatics.BreakHitResult` _outhit))
          (`GameplayStatics.ApplyDamage` _hitactor 0.6 (`self.OwningPlayerController`) self)
          (`GameplayStatics.SpawnSoundAtLocation` "/Game/TSS_Game/SFX/Melee/Impact_Punch_Harder01_Cue.Impact_Punch_Harder01_Cue" _location (struct) 1.0 1.0 0.0 null null)))
      (:`then_1`
        (`KismetSystemLibrary.Delay` 1.0)
        (set `self.IsMeleeAttacking` false)))))

(event `EnhancedInput|/Game/TSS_Game/Blueprints/EnhancedInput/InputAction_Melee`
  (params (ActionValue :type Boolean) (ElapsedSeconds :type "Float (double-precision)") (TriggeredSeconds :type "Float (double-precision)") (InputAction :type "InputAction Object Reference" :default "/Game/TSS_Game/Blueprints/EnhancedInput/InputAction_Melee.InputAction_Melee"))
  ;[1 1 1] Melee
  (:`Triggered`
    (`self.Server_Melee`)))

(event `EnhancedInput|/Game/TSS_Game/Blueprints/EnhancedInput/InputAction_Inventory`
  (params (ActionValue :type Boolean) (ElapsedSeconds :type "Float (double-precision)") (TriggeredSeconds :type "Float (double-precision)") (InputAction :type "InputAction Object Reference" :default "/Game/TSS_Game/Blueprints/EnhancedInput/InputAction_Inventory.InputAction_Inventory"))
  ;[1 1 1] Inventory
  (:`Triggered`
    (bind _returnvalue (`|CreateWidget` "/Game/TSS_Game/Blueprints/Inventory/W_Inventory_UI.W_Inventory_UI_C" (`self.OwningPlayerController`) self))
    (`UserWidget.AddToViewport` _returnvalue 0)))

(event `Equip_From_Inventory`
  (params (IndexInInventory :type Integer))
  ;[1 1 1] Inventory
  (`self.EquipWeapon` IndexInInventory))

(event `EnhancedInput|/Game/TSS_Game/Blueprints/EnhancedInput/InputAction_GrenadeThrow`
  (params (ActionValue :type Boolean) (ElapsedSeconds :type "Float (double-precision)") (TriggeredSeconds :type "Float (double-precision)") (InputAction :type "InputAction Object Reference" :default "/Game/TSS_Game/Blueprints/EnhancedInput/InputAction_GrenadeThrow.InputAction_GrenadeThrow"))
  (bind _plane (`self.Plane`))
  ;[1 1 1] Grenades
  (:`Started`
    (`SceneComponent.SetVisibility` _plane true false))
  (:`Completed`
    (`SceneComponent.SetVisibility` _plane false false)
    (`self.Server_Spawn_Grenade` (`SceneComponent.K2_GetComponentToWorld` (`self.BulletSpawnLocation`)) self)))

(event `Drop_From_Inventory`
  (params (SelectedWeapon :type "/Game/TSS_Game/Blueprints/Weapons/Base/BP_WeaponBase Object Reference") (AmmoCurrent :type Integer) (AmmoInReserve :type Integer))
  (bind _ut_inventory (`self.UT_Inventory`))
  ;[1 1 1] Inventory
  (bind _returnvalue (`|SpawnActorFromClass` (`GameplayStatics.GetObjectClass` SelectedWeapon) (`self.GetTransform`) "AlwaysSpawn" "SelectDefaultAtRuntime" null 1 100.0 0.0 1 10.0 20.0 null))
  (`/Engine/EditorBlueprintResources/StandardMacros.IsValid` _returnvalue
    (:`Is Valid`
      (`/Game/TSS_Game/Blueprints/Weapons/Base/BP_WeaponBase.Update_Stats_Server` _returnvalue AmmoCurrent AmmoInReserve)
      (`/Engine/EditorBlueprintResources/StandardMacros.IsValid` SelectedWeapon
        (:`Is Valid`
          (`KismetArrayLibrary.Array_RemoveItem` _ut_inventory SelectedWeapon)
          (`|ExecutionSequence`
            (:`then_0`
              (`self.K2_DestroyActor` SelectedWeapon))
            (:`then_1`
              (if (> (`KismetArrayLibrary.Array_Length` _ut_inventory) 0) :!label _label_5
                (`self.EquipWeapon` 0)))))
        (:`Is Not Valid`
          (goto _label_5))))))

(event `Server_Spawn_Grenade`
  (params (SpawnTransform :type "Transform Structure") (Instigator :type "Pawn Object Reference"))
  ;[1 1 1] Grenades
  (`self.Multicast_SpawnGrenade` SpawnTransform Instigator))

(event `Multicast_SpawnGrenade`
  (params (SpawnTransform :type "Transform Structure") (Instigator :type "Pawn Object Reference"))
  ;[1 1 1] Grenades
  (if (> (`self.Grenades`) 0)
    (`|SpawnActorFromClass` "/Game/TSS_Game/Blueprints/Weapons/BPC_GrenadeProjectile.BPC_GrenadeProjectile_C" SpawnTransform "AlwaysSpawn" "OverrideRootScale" null 100.0 Instigator)
    (set `self.Grenades` (- (`self.Grenades`) 1))
    (else
      (`KismetSystemLibrary.PrintString` "You don't have any more grenades"))))

(fn `AddExp`
  (params (`Exp to Add` :type Integer))
  (set `self.CurrentExp` (+ (`self.CurrentExp`) `Exp to Add`)))

(fn `AddWeapon`
  (params (WeaponToAdd :type "/Game/TSS_Game/Blueprints/Weapons/Base/BP_WeaponBase Object Reference (by ref)"))
  (returns (IndexOfTheAddedWeapon :type Integer))
  (bind _returnvalue (`KismetArrayLibrary.Array_Add` (`self.UT_Inventory`) WeaponToAdd))
  (return _returnvalue))

(fn `Blessings`)

(fn `Calculate Dash Target Location`
  (returns (Location :type "Vector Structure"))
  (bind _returnvalue (`self.GetLastMovementInputVector`))
  (return (+ (`self.K2_GetActorLocation`) (* (`KismetMathLibrary.SelectVector` (`self.GetActorForwardVector`) _returnvalue (== _returnvalue (0.0 0.0 0.0))) (`self.MaxDashDistance`)))))

(fn `CycleTroughInventory`
  (returns (NextIndex :type Integer))
  (bind _ut_inventory (`self.UT_Inventory`))
  (bind _returnvalue (`KismetArrayLibrary.Array_Find` _ut_inventory (`self.EquippedWeapon`)))
  (bind _returnvalue_2 (`KismetArrayLibrary.Array_LastIndex` _ut_inventory))
  (if (== _returnvalue _returnvalue_2)
    (set `self.IndexZero` 0)
    (else
      (set `self.IndexZero` (`KismetMathLibrary.Clamp` (+ _returnvalue 1) 0 _returnvalue_2))))
  (return (`self.IndexZero`)))

(fn `EquipWeapon`
  (params (IndexInInventory :type Integer))
  (for (_array_element _array_index) (`self.UT_Inventory`)
    (`/Engine/EditorBlueprintResources/StandardMacros.IsValid` _array_element
      (:`Is Valid`
        (`self.SetActorHiddenInGame` _array_element (!= _array_index IndexInInventory))
        (`/Game/TSS_Game/Blueprints/Weapons/Base/BP_WeaponBase.StopWeaponFire` _array_element))))
  (bind _output_get (set `self.EquippedWeapon` (`|GetArrayItem` (`self.UT_Inventory`) IndexInInventory)))
  (`/Engine/EditorBlueprintResources/StandardMacros.IsValid` _output_get
    (:`Is Valid`
      (`self.K2_AttachToComponent` _output_get (`self.Mesh`) "GripPoint" "SnapToTarget" "SnapToTarget" "SnapToTarget" true)
      (`/Game/TSS_Game/Blueprints/Weapons/Base/BP_WeaponBase.StopWeaponFire` _output_get))))

(fn `GetFurthestValidLocationAlongRoute`
  (params (Start :type "Vector Structure") (End :type "Vector Structure"))
  (returns (Location :type "Vector Structure"))
  (locals (Direction :type "Vector Structure" :default (0.0 0.0 0.0)) (CapsuleDiameter :type "Float (double-precision)") (CapsuleCount :type Integer) (CurrentCapsuleLocation :type "Vector Structure"))
  (bind (_outradius _outhalfheight) (`CapsuleComponent.GetUnscaledCapsuleSize` (`self.CapsuleComponent`)))
  (set `local.Direction` (`KismetMathLibrary.GetDirectionUnitVector` Start End))
  (bind _output_get (set `local.CapsuleDiameter` (* (`CapsuleComponent.CapsuleRadius` (`self.CapsuleComponent`)) 2.0)))
  (bind _output_get_2 (set `local.CapsuleCount` (/ (`KismetMathLibrary.Vector_Distance` Start End) _output_get)))
  (for _index (range (+ _output_get_2 1))
    (bind _output_get_3 (set `local.CurrentCapsuleLocation` (+ (`local.Start`) (* (- (`local.CapsuleCount`) _index) (`local.Direction`) (`local.CapsuleDiameter`)))))
    (bind _outhits (`KismetSystemLibrary.CapsuleTraceMultiForObjects` _output_get_3 _output_get_3 _outradius _outhalfheight (`|MakeArray` "ObjectTypeQuery1" "ObjectTypeQuery2" "ObjectTypeQuery3" "ObjectTypeQuery5" "ObjectTypeQuery6" :!type "EObjectTypeQuery Enum")))
    (bind _isvalid (`self.IsValidDashLocation` (`local.CurrentCapsuleLocation`) _outhits))
    (if _isvalid
      (return (`local.CurrentCapsuleLocation`))))
  (return (`local.Start`)))

(fn `IsValidDashLocation`
  (params (Location :type "Vector Structure") (Hits :type "Array of HitResult Structure"))
  (returns (IsValid :type Boolean))
  (bind (_outhit _returnvalue) (`KismetSystemLibrary.LineTraceSingle` Location (+ Location (0.0 0.0 -500.0)) "TraceTypeQuery1"))
  (if _returnvalue
    (if (`KismetArrayLibrary.Array_IsEmpty` Hits)
      (return true)
      (else
        (for _array_element Hits
          (if (`|EnumEquality` (`PrimitiveComponent.GetCollisionResponseToChannel` (`.HitComponent` (`GameplayStatics.BreakHitResult` _array_element)) "ECC_Pawn") "ECR_Block")
            _))
        (return true)))
    (else
      (return false))))

(fn `RemoveExp`
  (params (`Exp to Remove` :type Integer))
  (bind _currentexp (`self.CurrentExp`))
  (if (>= _currentexp `Exp to Remove`)
    (if (>= _currentexp 1)
      (set `self.CurrentExp` (`KismetMathLibrary.Clamp` (- _currentexp `Exp to Remove`) 0 999999)))))

(fn `SetControllerInputMode`
  (params (Controls :type "/Game/TSS_Game/Blueprints/System/E_Controls Enum" :default "NewEnumerator0"))
  (if (`self.IsLocallyControlled`)
    (bind _output_get (set `self.Controls` Controls))
    (switch `/Game/TSS_Game/Blueprints/System/E_Controls` _output_get
      (:`NewEnumerator0`
        (set `self.MouseRotationEnabled` true))
      (:`NewEnumerator1`
        (set `self.MouseRotationEnabled` false)))))

(fn `SpawnWeapon`
  (params (Class :type "/Game/TSS_Game/Blueprints/Weapons/Base/BP_WeaponBase Class Reference"))
  (if (`KismetSystemLibrary.IsValidClass` Class)
    (`/Engine/EditorBlueprintResources/ActorMacros.Switch Has Authority`
      (:`Authority`
        (bind _returnvalue (`|SpawnActorFromClass` Class (`KismetMathLibrary.MakeTransform` (`SceneComponent.K2_GetComponentLocation` (`self.Mesh`))) "AlwaysSpawn" "OverrideRootScale" self 1 100.0 0.0 1 10.0 20.0 null))
        (message `/Game/TSS_Game/Blueprints/System/BPI_Interactive.InteractWithWeapon` _returnvalue self)
        (`/Game/TSS_Game/Blueprints/Weapons/Base/BP_WeaponBase.Update_Stats_Server` _returnvalue (`/Game/TSS_Game/Blueprints/Weapons/Base/BP_WeaponBase.AmmoCurrent` _returnvalue) (`/Game/TSS_Game/Blueprints/Weapons/Base/BP_WeaponBase.AmmoInReserve` _returnvalue))))))

(fn `UserConstructionScript`
  (set `self.AvailableDashCount` (`self.MaxDashCount`)))