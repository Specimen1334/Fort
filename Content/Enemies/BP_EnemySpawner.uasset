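; Enemy spawner that populates navigable ground around the player with basic, tank and swarmer AI enemies, escalating over time.
; Looping timers drive each type, spawning only while its live actor count is below a cap derived from MaxEnemies.
; Swarmers arrive in batches of ten, each call rolling its own random point.
; A difficulty timer increments a counter and multiplies MaxEnemies by it, so the caps compound.
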(event `EnemyDifficulty`
  (bind _output_get (set `self.DifficultyCounter` (+ (`self.DifficultyCounter`) 1.0)))
  (bind _output_get_2 (set `self.MaxEnemies` (* _output_get (`self.MaxEnemies`)))))

(event `self.ReceiveBeginPlay`
  (`KismetSystemLibrary.K2_SetTimer` null "SpawnEnemies" 1.0 true)
  (`KismetSystemLibrary.K2_SetTimer` null "SpawnTank" 30.0 true)
  (`KismetSystemLibrary.K2_SetTimer` null "SpawnSwarmer" 60.0 true)
  (`KismetSystemLibrary.K2_SetTimer` null "EnemyDifficulty" 30.0 true)
  (`KismetSystemLibrary.K2_SetTimer` null "SpawnSwarmer" 60.0 true)
  (`KismetSystemLibrary.K2_SetTimer` null "SpawnSwarmer" 60.0 true))

(event `SpawnEnemies`
  (bind _outactors (`GameplayStatics.GetAllActorsOfClass` "/Game/Enemies/BP_Basic.BP_Basic_C"))
  (if (< (`KismetArrayLibrary.Array_Length` _outactors) (`KismetMathLibrary.FTrunc` (stale `EnemyDifficulty` _output_get_2)))
    (`AIBlueprintHelperLibrary.SpawnAIFromClass` "/Game/Enemies/BP_Basic.BP_Basic_C" null (`NavigationSystemV1.K2_GetRandomReachablePointInRadius` (`self.K2_GetActorLocation` (`GameplayStatics.GetPlayerCharacter` 0)) 5000.0 null null) (struct) false null)))

(event `SpawnTank`
  (bind _outactors (`GameplayStatics.GetAllActorsOfClass` "/Game/Enemies/BP_TankEnemy.BP_TankEnemy_C"))
  (if (< (`KismetArrayLibrary.Array_Length` _outactors) (`KismetMathLibrary.FTrunc` (/ (stale `EnemyDifficulty` _output_get_2) 10.0)))
    (`AIBlueprintHelperLibrary.SpawnAIFromClass` "/Game/Enemies/BP_TankEnemy.BP_TankEnemy_C" null (`NavigationSystemV1.K2_GetRandomReachablePointInRadius` (`self.K2_GetActorLocation` (`GameplayStatics.GetPlayerCharacter` 0)) 5000.0 null null) (struct) false null)))

(event `SpawnSwarmer`
  (bind _randomlocation (`NavigationSystemV1.K2_GetRandomReachablePointInRadius` (`self.K2_GetActorLocation` (`GameplayStatics.GetPlayerCharacter` 0)) 5000.0 null null))
  (bind _randomlocation_2 (`NavigationSystemV1.K2_GetRandomReachablePointInRadius` _randomlocation 5.0 null null))
  (bind _outactors (`GameplayStatics.GetAllActorsOfClass` "/Game/Enemies/BP_SwarmerEnemy.BP_SwarmerEnemy_C"))
  (if (< (`KismetArrayLibrary.Array_Length` _outactors) (`KismetMathLibrary.FTrunc` (* (stale `EnemyDifficulty` _output_get_2) 2.0)))
    (`AIBlueprintHelperLibrary.SpawnAIFromClass` "/Game/Enemies/BP_SwarmerEnemy.BP_SwarmerEnemy_C" null _randomlocation (struct) false null)
    (`AIBlueprintHelperLibrary.SpawnAIFromClass` "/Game/Enemies/BP_SwarmerEnemy.BP_SwarmerEnemy_C" null _randomlocation_2 (struct) false null)
    (`AIBlueprintHelperLibrary.SpawnAIFromClass` "/Game/Enemies/BP_SwarmerEnemy.BP_SwarmerEnemy_C" null _randomlocation_2 (struct) false null)
    (`AIBlueprintHelperLibrary.SpawnAIFromClass` "/Game/Enemies/BP_SwarmerEnemy.BP_SwarmerEnemy_C" null _randomlocation_2 (struct) false null)
    (`AIBlueprintHelperLibrary.SpawnAIFromClass` "/Game/Enemies/BP_SwarmerEnemy.BP_SwarmerEnemy_C" null _randomlocation_2 (struct) false null)
    (`AIBlueprintHelperLibrary.SpawnAIFromClass` "/Game/Enemies/BP_SwarmerEnemy.BP_SwarmerEnemy_C" null _randomlocation_2 (struct) false null)
    (`AIBlueprintHelperLibrary.SpawnAIFromClass` "/Game/Enemies/BP_SwarmerEnemy.BP_SwarmerEnemy_C" null _randomlocation_2 (struct) false null)
    (`AIBlueprintHelperLibrary.SpawnAIFromClass` "/Game/Enemies/BP_SwarmerEnemy.BP_SwarmerEnemy_C" null _randomlocation_2 (struct) false null)
    (`AIBlueprintHelperLibrary.SpawnAIFromClass` "/Game/Enemies/BP_SwarmerEnemy.BP_SwarmerEnemy_C" null _randomlocation_2 (struct) false null)
    (`AIBlueprintHelperLibrary.SpawnAIFromClass` "/Game/Enemies/BP_SwarmerEnemy.BP_SwarmerEnemy_C" null _randomlocation_2 (struct) false null)))

(fn `UserConstructionScript`)