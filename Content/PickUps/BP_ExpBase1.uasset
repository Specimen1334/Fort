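; Experience pickup actor that labels itself with its ExpName text, held at a fixed world rotation to suit the camera.
; Each Tick it checks the distance to the player's BP_CharacterBase and, within the Magnet radius, glides toward it with a frame-rate-dependent VInterpTo.
; At close range it grants a hardcoded amount of experience through AddExp and destroys itself, using distance checks rather than overlap events.
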(event `self.ReceiveBeginPlay`
  (`TextRenderComponent.K2_SetText` (`self.Exp_TXT`) (`self.ExpName`)))

(event `self.ReceiveTick`
  (params (DeltaSeconds :type "Float (single-precision)"))
  (`SceneComponent.K2_SetWorldRotation` (`self.Exp_TXT`) (struct :`Pitch` 45.0 :`Yaw` 180.0) false false) ; Rotates the text to face the camera
  (bind _asbp_character_base (cast `/Game/Characters/BP_CharacterBase` (`GameplayStatics.GetPlayerCharacter` 0)))
  (if (< (`self.GetDistanceTo` _asbp_character_base) (`self.Magnet`))
    (`SceneComponent.K2_SetWorldLocation` (`self.DefaultSceneRoot`) (`KismetMathLibrary.VInterpTo` (`self.K2_GetActorLocation`) (`self.K2_GetActorLocation` _asbp_character_base) 1.0 0.05) true false)
    (if (< (`self.GetDistanceTo` _asbp_character_base) 100.0)
      (`/Game/Characters/BP_CharacterBase.AddExp` _asbp_character_base 100)
      (`self.K2_DestroyActor`))))

(event `self.ReceiveActorBeginOverlap`
  (params (OtherActor :type "Actor Object Reference")))

(fn `UserConstructionScript`)