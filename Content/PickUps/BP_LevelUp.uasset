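; BP_LevelUp is an overlap-triggered level-up point that spends a character's experience to upgrade their equipped weapon.
; On overlap with a BP_CharacterBase, it scales BaseExpCost by the square of the weapon level.
; If affordable, it raises the level, deducts the cost and calls RandomStatBoost, staying in the world afterward.
; A text label shows LevelName, reset every Tick to a fixed camera-facing rotation.
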(event `self.ReceiveBeginPlay`
  (`TextRenderComponent.K2_SetText` (`self.Level_TXT`) (`self.LevelName`)))

(event `self.ReceiveTick`
  (params (DeltaSeconds :type "Float (single-precision)"))
  (`SceneComponent.K2_SetWorldRotation` (`self.Level_TXT`) (struct :`Pitch` 45.0 :`Yaw` 180.0) false false) ; Rotates the text to face the camera
)

(event `self.ReceiveActorBeginOverlap`
  (params (OtherActor :type "Actor Object Reference"))
  (bind _asbp_character_base (cast `/Game/Characters/BP_CharacterBase` OtherActor))
  (bind _equippedweapon (`/Game/Characters/BP_CharacterBase.EquippedWeapon` _asbp_character_base))
  (bind _weaponlevel (`/Game/TSS_Game/Blueprints/Weapons/Base/BP_WeaponBase.WeaponLevel` _equippedweapon))
  (bind _output_get (set `self.RequiredExp` (* (`self.BaseExpCost`) (* _weaponlevel _weaponlevel))))
  (`KismetSystemLibrary.PrintString` (`KismetStringLibrary.Conv_DoubleToString` _output_get))
  (if (>= (`/Game/Characters/BP_CharacterBase.CurrentExp` _asbp_character_base) _output_get)
    (bind _output_get_2 (set `/Game/TSS_Game/Blueprints/Weapons/Base/BP_WeaponBase.WeaponLevel` (+ (`/Game/TSS_Game/Blueprints/Weapons/Base/BP_WeaponBase.WeaponLevel` _equippedweapon) 1.0) _equippedweapon))
    (`KismetSystemLibrary.PrintString` (`KismetStringLibrary.Conv_DoubleToString` _output_get_2) true true (struct :`G` 0.66 :`B` 1.0 :`A` 1.0) 60.0)
    (set `/Game/Characters/BP_CharacterBase.CurrentExp` (`KismetMathLibrary.FTrunc` (- (`/Game/Characters/BP_CharacterBase.CurrentExp` _asbp_character_base) (`self.RequiredExp`))) _asbp_character_base)
    (`/Game/TSS_Game/Blueprints/Weapons/Base/BP_WeaponBase.Random Stat Boost` _equippedweapon)))

(fn `UserConstructionScript`)