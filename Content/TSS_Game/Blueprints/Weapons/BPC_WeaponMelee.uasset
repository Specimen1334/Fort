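; Melee weapon Blueprint that turns the Fire event into an axe swing by the owning player character.
; Fire routes through server and multicast events to play the swing montage, then runs a short forward sphere trace from the capsule after a brief delay.
; Hits take damage and play an impact sound, with a blood-style particle burst for Enemy-tagged actors, while a boolean gate blocks overlapping swings.
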(event `Server_Melee`
  (`self.Multi_Melee`))

(event `Multi_Melee`
  (bind _playercast (`self.PlayerCast`))
  (bind _playercast_2 (`self.PlayerCast`))
  (bind _returnvalue (+ (`SceneComponent.K2_GetComponentLocation` (`Character.CapsuleComponent` _playercast_2)) (0.0 0.0 5.0)))
  (if (not (`self.NewVar_0_0`))
    (set `self.NewVar_0_0` true)
    (`AnimInstance.Montage_Play` (`SkeletalMeshComponent.GetAnimInstance` (`Character.Mesh` _playercast_2)) "/Game/TSS_Game/Character/AnimStarterPack/ActionRPG/Anim_Axe_Combat_Swing_Montage.Anim_Axe_Combat_Swing_Montage" 1.0 "Duration" 0.0 true) ; Change character montage here
    (`KismetSystemLibrary.Delay` 0.2)
    (bind (_outhit _returnvalue_2) (`KismetSystemLibrary.SphereTraceSingle` _returnvalue (+ _returnvalue (* (`KismetMathLibrary.GetForwardVector` (`self.K2_GetActorRotation` _playercast_2)) 150.0)) 30.0 "TraceTypeQuery1" false (`/Game/Characters/BP_CharacterBase.UT_Inventory` _playercast)))
    (if _returnvalue_2
      (bind (_bblockinghit _binitialoverlap _time _distance _location _impactpoint _normal _impactnormal _physmat _hitactor) (`GameplayStatics.BreakHitResult` _outhit))
      (`GameplayStatics.ApplyDamage` _hitactor 1.0 (`/Game/Characters/BP_CharacterBase.OwningPlayerController` _playercast) _playercast)
      (`GameplayStatics.SpawnSoundAtLocation` "/Game/TSS_Game/SFX/Melee/Impact_Punch_Harder01_Cue.Impact_Punch_Harder01_Cue" _location (struct) 1.0 1.0 0.0 null null)
      (if (`self.ActorHasTag` _hitactor "Enemy")
        (`GameplayStatics.SpawnEmitterAtLocation` "/Game/TSS_Game/Particles/P_body_bullet_impact.P_Body_Bullet_Impact" _location (struct) (3.0 3.0 3.0))))
    (`KismetSystemLibrary.Delay` 0.2)
    (set `self.NewVar_0_0` false)))

(event `self.Fire`
  (`self.Server_Melee`))

(fn `UserConstructionScript`
  (`parent.UserConstructionScript`))