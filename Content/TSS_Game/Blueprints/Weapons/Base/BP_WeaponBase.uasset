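; Base weapon actor that shows its name until picked up, then equips to the interacting character and fires projectiles.
; Server-side Fire is rate-gated, uses a looping timer for automatic weapons, checks ammo or reloads via montage, and multicasts muzzle effects.
; Levelling derives damage, cooldown, area and projectile count from weapon level and nearest character's stats, with special cases for Cauldron and Galatine projectiles.
; RandomStatBoost randomly improves base stats.
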(event `self.ReceiveTick`
  (params (DeltaSeconds :type "Float (single-precision)"))
  ;[1 1 1] Tick
  (if (not (`self.isTaken`))
    (`SceneComponent.K2_SetWorldRotation` (`self.WeaponNameText`) (struct :`Pitch` 45.0 :`Yaw` 180.0) false false) ; Rotates the text to face the camera
  ))

(event `self.ReceiveBeginPlay`
  (bind _weaponnametext (`self.WeaponNameText`))
  ;[1 1 1] Begin Play
  (set `self.SpawnedWeapon` self)
  (set `self.AmmoCurrent` (`self.AmmoMax`))
  (set `self.AmmoInReserveMax` (`self.AmmoInReserve`))
  (if (`self.isTaken`)
    (`TextRenderComponent.K2_SetText` _weaponnametext (`KismetTextLibrary.Conv_StringToText` " "))
    (else
      (`TextRenderComponent.K2_SetText` _weaponnametext (`self.WeaponName`)))))

(event `/Game/TSS_Game/Blueprints/System/BPI_Interactive.InteractWithWeapon`
  (params (CharacterReference :type "/Game/Characters/BP_CharacterBase Object Reference"))
  ;[1 1 1] Event interact
  ;[1 1 1] Equip
  (if (not (`self.isTaken`))
    (set `self.PlayerCast` CharacterReference)
    (`self.AddAndEquip` CharacterReference)))

(event `MultiPlayMontage`
  (bind _playercast (`self.PlayerCast`))
  ;[1 1 1] Equip
  (`/Engine/EditorBlueprintResources/StandardMacros.IsValid` _playercast
    (:`Is Valid`
      (set `/Game/Characters/BP_CharacterBase.isSwitchingWeapons` true _playercast)
      (bind _returnvalue (`AnimInstance.Montage_Play` (`SkeletalMeshComponent.GetAnimInstance` (`Character.Mesh` _playercast)) "/Game/TSS_Game/Character/AnimStarterPack/Equip_Rifle_Standing_Montage.Equip_Rifle_Standing_Montage" 2.0 "Duration" 0.0 true))
      (`KismetSystemLibrary.Delay` _returnvalue)
      (set `/Game/Characters/BP_CharacterBase.isSwitchingWeapons` false _playercast))))

(event `MulticastShowText`
  ;[1 1 1] Equip
  (`TextRenderComponent.K2_SetText` (`self.WeaponNameText`) (`KismetTextLibrary.Conv_StringToText` " ")))

(event `AddAndEquip`
  (params (CharacterReference :type "/Game/Characters/BP_CharacterBase Object Reference"))
  ;[1 1 1] Equip
  (bind _indexoftheaddedweapon (`/Game/Characters/BP_CharacterBase.AddWeapon` CharacterReference (`self.SpawnedWeapon`)))
  (`/Game/Characters/BP_CharacterBase.EquipWeapon` CharacterReference _indexoftheaddedweapon)
  (`PrimitiveComponent.SetCollisionEnabled` (`self.Sphere`) "NoCollision")
  (set `self.isTaken` true)
  (`self.MulticastShowText`)
  (`self.MultiPlayMontage`))

(event `Fire`
  (bind (_atkdamage _cooldown _area _noproj) (`self.Levelling`))
  (bind _playercast (`self.PlayerCast`))
  (bind (_returnvalue_location _returnvalue_rotation) (`self.CalculateSpawnLocation` (`self.SpawnFromCharacter`)))
  ;[1 1 1] Fire - Runs on the Server (called from Character)
  (`/Engine/EditorBlueprintResources/StandardMacros.DoOnce` false :!label _label
    (:`Completed`
      (`|ExecutionSequence`
        (:`then_0`
          (if (`self.isReloading`)
            _
            (elif (`self.Automatic`)
              (`self.FireWeaponStarted`)
              (`KismetSystemLibrary.K2_SetTimer` null "FireWeaponStarted" _cooldown true)
              (elif (`self.InfiniteAmmo`)
                (if (not (`/Game/Characters/BP_CharacterBase.IsDead` (`self.PlayerCast`))) :!label _label_2
                  (for _index (range (+ _noproj 1))
                    (`|SpawnActorFromClass` (`self.ProjectileToFire`) (`KismetMathLibrary.MakeTransform` (+ _returnvalue_location (* _index (0.0 0.0 20.0))) _returnvalue_rotation _area) "AlwaysSpawn" "OverrideRootScale" (`/Game/Characters/BP_CharacterBase.OwningPlayerController` _playercast) _atkdamage _playercast))
                  ;[1 1 1] Happens on all Clients
                  (`self.FireMulticastEvent`))
                (else
                  (bind _canfire (`self.AmmoCheck` :!label _label_3))
                  (if _canfire
                    (goto _label_2)
                    (else
                      (`self.Reload`))))))))
        (:`then_1`
          (`KismetSystemLibrary.RetriggerableDelay` (`self.DelayBetweenShots`))
          (goto _label :!via `Reset`))))))

(event `FireMulticastEvent`
  ;[1 1 1] Happens on all Clients
  (`GameplayStatics.SpawnSoundAtLocation` (`self.FiringSound`) (`self.K2_GetActorLocation`) (struct) 1.0 1.0 0.0 null null) ; Firing Sound
  (`GameplayStatics.SpawnEmitterAttached` (`self.FiringEffect`) (`self.WeaponMesh`) (`self.MuzzleSocketName`) (0.0 0.0 0.0) (struct) (1.0 1.0 1.0) "SnapToTarget") ; Particle
)

(event `FireWeaponStarted`
  ;[1 1 1] Fire - Runs on the Server (called from Character)
  (if (`self.InfiniteAmmo`)
    (goto _label_2)
    (else
      (goto _label_3))))

(event `StopWeaponFire`
  ;[1 1 1] Fire - Runs on the Server (called from Character)
  (`KismetSystemLibrary.K2_ClearTimer` null "FireWeaponStarted"))

(event `Reload`
  ;[1 1 1] Reloading
  (`KismetSystemLibrary.K2_ClearTimer` null "FireWeaponStarted")
  (bind _canreload (`self.AmmoCheckMag`))
  (if _canreload
    (if (not (`self.isReloading`))
      (set `self.isReloading` true)
      (bind _returnvalue (`AnimInstance.Montage_Play` (`SkeletalMeshComponent.GetAnimInstance` (`Character.Mesh` (`self.PlayerCast`))) (`self.ReloadAnimMontage`) 1.0 "MontageLength" 0.0 true))
      (`KismetSystemLibrary.Delay` _returnvalue)
      (`self.AmmoReload`)
      (set `self.isReloading` false))))

(event `Update_Stats_Server`
  (params (AmmoCurrent :type Integer) (AmmoInReserve :type Integer))
  (set `self.AmmoCurrent` AmmoCurrent)
  (set `self.AmmoInReserve` AmmoInReserve))

(event `Random Stat Boost`
  (bind _returnvalue (`KismetMathLibrary.FTrunc` (`KismetMathLibrary.RandomFloatInRange` 1.0 3.9)))
  (if (== _returnvalue 1)
    (set `self.StartDamage` (+ (`self.StartDamage`) 50.0))
    (elif (== _returnvalue 2)
      (set `self.BaseCooldown` (- (`self.BaseCooldown`) 0.1))
      (elif (== _returnvalue 3)
        (set `self.BaseAoe` (+ (`self.BaseAoe`) (0.0 0.1 0.0)))))))

(fn `AmmoCheck`
  (returns (CanFire :type Boolean))
  (if (> (`self.AmmoCurrent`) 0)
    (set `self.AmmoCurrent` (`KismetMathLibrary.Clamp` (- (- (`self.AmmoCurrent`) 1) (`self.AdditionalProjectilesToFire`)) 0 (`self.AmmoInReserveMax`)))
    (return true)
    (else
      (set `self.AmmoCurrent` 0)
      (return false))))

(fn `AmmoCheckMag`
  (returns (CanReload :type Boolean))
  (return (and (>= (`self.AmmoInReserve`) 1) (< (`self.AmmoCurrent`) (`self.AmmoMax`)))))

(fn `AmmoReload`
  (bind _zero (`self.Zero`))
  (bind _output_get (set `self.AmmoNeeded` (- (`self.AmmoMax`) (`self.AmmoCurrent`))))
  (`/Engine/EditorBlueprintResources/StandardMacros.CompareInt` (`self.AmmoInReserve`) (`self.AmmoMax`)
    (:`>`
      (set `self.AmmoCurrent` (`self.AmmoMax`) :!label _label))
    (:`==`
      (goto _label))
    (:`<`
      (set `self.AmmoCurrent` (`KismetMathLibrary.Clamp` (+ (`self.AmmoCurrent`) (`self.AmmoInReserve`)) (`self.Zero`) (`self.AmmoMax`)))))
  (bind _returnvalue (- (`self.AmmoInReserve`) _output_get))
  (`/Engine/EditorBlueprintResources/StandardMacros.CompareInt` _returnvalue _zero
    (:`>`
      (set `self.AmmoInReserve` _returnvalue))
    (:`==`
      (set `self.AmmoInReserve` _zero :!label _label_2))
    (:`<`
      (goto _label_2))))

(fn `CalculateSpawnLocation`
  (params (SpawnFromCharacter :type Boolean))
  (returns (ReturnValue_Location :type "Vector Structure") (ReturnValue_Rotation :type "Rotator Structure"))
  (bind _playercast (`self.PlayerCast`))
  (bind _returnvalue_location (`KismetMathLibrary.BreakTransform` (`SceneComponent.GetSocketTransform` (`self.WeaponMesh`) (`self.MuzzleSocketName`) "RTS_World")))
  (bind _returnvalue (+ (`self.Spread`) (`self.AdditionalProjectilesToFire`)))
  (bind (_returnvalue_location_2 _returnvalue_rotation) (`KismetMathLibrary.BreakTransform` (`SceneComponent.K2_GetComponentToWorld` (`/Game/Characters/BP_CharacterBase.BulletSpawnLocation` _playercast))))
  (bind (_returnvalue_roll _returnvalue_pitch _returnvalue_yaw) (`KismetMathLibrary.BreakRotator` (select `bool` SpawnFromCharacter :`false` (`Pawn.GetControlRotation` _playercast) :`true` _returnvalue_rotation)))
  (return (select `bool` SpawnFromCharacter :`false` _returnvalue_location :`true` _returnvalue_location_2) (`KismetMathLibrary.MakeRotator` _returnvalue_roll _returnvalue_pitch (select `bool` SpawnFromCharacter :`false` (+ _returnvalue_yaw (`KismetMathLibrary.RandomFloatInRange` (* _returnvalue -1.0) _returnvalue)) :`true` _returnvalue_yaw :!type "Float (double-precision)"))))

(fn `Levelling`
  (returns (AtkDamage :type "Float (double-precision)") (Cooldown :type "Float (double-precision)") (Area :type "Vector Structure") (NoProj :type Integer))
  (bind _baseaoe (`self.BaseAoe`))
  (bind _outactors (`GameplayStatics.GetAllActorsOfClass` "/Game/Characters/BP_CharacterBase.BP_CharacterBase_C"))
  (bind _asbp_character_base (cast `/Game/Characters/BP_CharacterBase` (`.ReturnValue` (`GameplayStatics.FindNearestActor` (`self.K2_GetActorLocation`) _outactors))))
  (if (== (`self.ProjectileToFire`) "/Game/Weapons/BP_ProjCauldron.BP_ProjCauldron_C")
    (bind _output_get (set `self.AdditionalProjectilesToFire` (`KismetMathLibrary.FTrunc` (- (+ (`self.BaseProjectiles`) (* (`self.WeaponLevel`) 2.0)) 2.0)))))
  (bind _returnvalue (- (`self.BaseCooldown`) (* (`self.WeaponLevel`) 0.1) (`/Game/Characters/BP_CharacterBase.PlayerCooldown` _asbp_character_base)))
  (if (<= _returnvalue 0.0)
    (set `self.Cooldown` 0.1)
    (else
      (bind _output_get_2 (set `self.Cooldown` _returnvalue))))
  (bind _output_get_3 (set `self.AtkDamage` (+ (* (* (`self.StartDamage`) (/ (`self.WeaponLevel`) 2.0)) (`/Game/Characters/BP_CharacterBase.PlayerDamage` _asbp_character_base)) 50.0)))
  (bind (_returnvalue_x _returnvalue_y _returnvalue_z) (`KismetMathLibrary.BreakVector` (+ _baseaoe (`KismetMathLibrary.MakeVector` 0.0 (* (`self.WeaponLevel`) 0.1)) (- (`/Game/Characters/BP_CharacterBase.PlayerAoe` _asbp_character_base) (1.0 1.0 1.0)))))
  (bind (_returnvalue_x_2 _returnvalue_y_2 _returnvalue_z_2) (`KismetMathLibrary.BreakVector` (select `bool` (== (`self.ProjectileToFire`) "/Game/Weapons/BP_ProjGalatine.BP_ProjGalatine_C") :`false` _baseaoe :`true` (`KismetMathLibrary.MakeVector` _returnvalue_x _returnvalue_y _returnvalue_z))))
  (return _output_get_3 _output_get_2 (`KismetMathLibrary.MakeVector` _returnvalue_x_2 _returnvalue_y_2 _returnvalue_z_2) _output_get))

(fn `UserConstructionScript`)