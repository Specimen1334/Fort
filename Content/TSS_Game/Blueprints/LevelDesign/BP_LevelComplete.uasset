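; BP_LevelComplete is a level exit volume that loads the next map once all players are inside it.
; Box overlaps by BP_CharacterBase actors adjust a counter, clamped and compared to the GameState PlayerArray length.
; On a full count it shows W_Loading for the first player controller, then after a brief delay calls MapTravel on BP_GameInstanceWithSettings with NextLevelMapName.
; A graph note says travel uses ServerTravel and only works in shipping builds.
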(event `self.Box.OnComponentBeginOverlap`
  (params (OverlappedComponent :type "PrimitiveComponent Object Reference") (OtherActor :type "Actor Object Reference") (OtherComp :type "PrimitiveComponent Object Reference") (OtherBodyIndex :type Integer) (bFromSweep :type Boolean) (SweepResult :type "HitResult Structure (by ref)"))
  ;[1 1 1] Checks if all players are inside the level exit volume
  (cast `/Game/Characters/BP_CharacterBase` OtherActor)
  (bind _allplayerspresent (`self.PlayerOverlapCalculation` true))
  (if _allplayerspresent
    (`KismetSystemLibrary.PrintString` "All players present")
    ;[1 1 1] Shows loading screen and loads the next map (uses ServerTravel and only works in a shipping build)
    (bind _returnvalue (`|CreateWidget` "/Game/TSS_Game/UI/W_Loading.W_Loading_C" (`GameplayStatics.GetPlayerController` 0)))
    (`/Engine/EditorBlueprintResources/StandardMacros.IsValid` _returnvalue
      (:`Is Valid`
        (`UserWidget.AddToViewport` _returnvalue 0)
        (`KismetSystemLibrary.Delay` 0.2)
        (bind _asbp_game_instance_with_settings (cast `/Game/TSS_Game/Blueprints/GameInstanceSettings/BP_GameInstanceWithSettings` (`GameplayStatics.GetGameInstance`)))
        (`/Game/TSS_Game/Blueprints/GameInstanceSettings/BP_GameInstanceWithSettings.MapTravel` _asbp_game_instance_with_settings (`self.NextLevelMapName`))))
    (else
      (`KismetSystemLibrary.PrintString` "Missing player"))))

(event `self.Box.OnComponentEndOverlap`
  (params (OverlappedComponent :type "PrimitiveComponent Object Reference") (OtherActor :type "Actor Object Reference") (OtherComp :type "PrimitiveComponent Object Reference") (OtherBodyIndex :type Integer))
  ;[1 1 1] Checks if all players are inside the level exit volume
  (cast `/Game/Characters/BP_CharacterBase` OtherActor)
  (bind _allplayerspresent (`self.PlayerOverlapCalculation` false))
  (if (not _allplayerspresent)
    (`KismetSystemLibrary.PrintString` "Missing player")))

(fn `PlayerOverlapCalculation`
  (params (BeginOverlap :type Boolean))
  (returns (AllPlayersPresent :type Boolean))
  (if BeginOverlap
    (bind _output_get (set `self.PlayerOverlap` (`KismetMathLibrary.Clamp` (+ (`self.PlayerOverlap`) 1) 0 (`KismetArrayLibrary.Array_Length` (`GameStateBase.PlayerArray` (`GameplayStatics.GetGameState`))))))
    (return (== _output_get (`KismetArrayLibrary.Array_Length` (`GameStateBase.PlayerArray` (`GameplayStatics.GetGameState`)))))
    (else
      (bind _output_get_2 (set `self.PlayerOverlap` (`KismetMathLibrary.Clamp` (- (`self.PlayerOverlap`) 1) 0 (`KismetArrayLibrary.Array_Length` (`GameStateBase.PlayerArray` (`GameplayStatics.GetGameState`))))))
      (return (== _output_get_2 (`KismetArrayLibrary.Array_Length` (`GameStateBase.PlayerArray` (`GameplayStatics.GetGameState`))))))))

(fn `UserConstructionScript`)