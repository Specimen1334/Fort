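; BP_House is a level design house actor that hides its roof while characters are inside its overlap area.
; When a Character begins overlapping, it turns MeshRoof invisible.
; When a Character leaves, it restores the roof only if no BP_CharacterBase actors still overlap, so the roof stays hidden while any of them remain.
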(event `self.ReceiveActorBeginOverlap`
  (params (OtherActor :type "Actor Object Reference"))
  (cast `Character` OtherActor)
  (`SceneComponent.SetVisibility` (`self.Mesh_Roof`) false false))

(event `self.ReceiveActorEndOverlap`
  (params (OtherActor :type "Actor Object Reference"))
  (cast `Character` OtherActor)
  (if (not (> (`KismetArrayLibrary.Array_Length` (`self.GetOverlappingActors` "/Game/Characters/BP_CharacterBase.BP_CharacterBase_C")) 0))
    (`SceneComponent.SetVisibility` (`self.Mesh_Roof`) true false)))

(fn `UserConstructionScript`)