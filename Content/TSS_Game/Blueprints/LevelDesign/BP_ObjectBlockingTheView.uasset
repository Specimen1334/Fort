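; BP_ObjectBlockingTheView is a level-design actor whose mesh turns transparent while a character overlaps it, presumably so it stops blocking the view.
; On BeginPlay it caches the mesh's original materials.
; When a Character begins overlapping, every material slot is swapped to M_Transparent.
; When a Character leaves, the cached materials are restored only if no BP_CharacterBase actors still overlap.
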(event `self.ReceiveBeginPlay`
  (for _array_element (`MeshComponent.GetMaterials` (`self.Mesh`))
    (`KismetArrayLibrary.Array_Add` (`self.Original_Material`) _array_element)))

(event `self.ReceiveActorBeginOverlap`
  (params (OtherActor :type "Actor Object Reference"))
  (bind _mesh (`self.Mesh`))
  (cast `Character` OtherActor)
  (for (_ _array_index) (`MeshComponent.GetMaterials` _mesh)
    (`PrimitiveComponent.SetMaterial` _mesh _array_index "/Game/TSS_Game/Materials/M_Transparent.M_Transparent")))

(event `self.ReceiveActorEndOverlap`
  (params (OtherActor :type "Actor Object Reference"))
  (cast `Character` OtherActor)
  (if (not (> (`KismetArrayLibrary.Array_Length` (`self.GetOverlappingActors` "/Game/Characters/BP_CharacterBase.BP_CharacterBase_C")) 0))
    (for (_array_element _array_index) (`self.Original_Material`)
      (`PrimitiveComponent.SetMaterial` (`self.Mesh`) _array_index _array_element))))

(fn `UserConstructionScript`)