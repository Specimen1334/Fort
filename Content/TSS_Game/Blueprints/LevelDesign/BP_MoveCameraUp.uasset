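; BP_MoveCameraUp is a level design trigger that swings the character camera to a top-down view while a BP_CharacterBase overlaps it.
; On begin overlap, a timeline lerps the character's spring arm from an angled pitch to straight down.
; On end overlap, a second timeline lerps it back, each playing from start with fixed endpoints.
; Spring arm length blends are present but disconnected, so only rotation changes.
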(event `self.ReceiveBeginPlay`)

(event `self.ReceiveActorBeginOverlap`
  (params (OtherActor :type "Actor Object Reference"))
  (bind _asbp_character_base (cast `/Game/Characters/BP_CharacterBase` OtherActor))
  (bind (_direction _alpha) (`Timeline|Timeline_Springarm` :!via `PlayFromStart`)
    (:`Update`
      (`SceneComponent.K2_SetRelativeRotation` (`/Game/Characters/BP_CharacterBase.SpringArm` _asbp_character_base) (`KismetMathLibrary.RLerp` (struct :`Pitch` -35.0) (struct :`Pitch` -90.0) _alpha) false false))))

(event `self.ReceiveActorEndOverlap`
  (params (OtherActor :type "Actor Object Reference"))
  (bind _asbp_character_base (cast `/Game/Characters/BP_CharacterBase` OtherActor))
  (bind (_direction _alpha) (`Timeline|Timeline_0` :!via `PlayFromStart`)
    (:`Update`
      (`SceneComponent.K2_SetRelativeRotation` (`/Game/Characters/BP_CharacterBase.SpringArm` _asbp_character_base) (`KismetMathLibrary.RLerp` (struct :`Pitch` -90.0) (struct :`Pitch` -35.0) _alpha) false false))))

(fn `UserConstructionScript`)