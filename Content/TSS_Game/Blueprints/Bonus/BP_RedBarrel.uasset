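; BP_RedBarrel is a physics-simulated barrel in the Bonus folder that reacts to any damage.
; On damage it activates its particle system at once and, after a two-second delay, spawns another actor at its location and destroys itself.
; Both reactions pass through Server events into Multicast events, so the particle activation, spawn and destruction are meant to run on every client.
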(event `self.ReceiveBeginPlay`
  (`PrimitiveComponent.SetSimulatePhysics` (`self.Cylinder`) true))

(event `Multicast_Spawn`
  (`|SpawnActorFromClass` null (`KismetMathLibrary.MakeTransform` (`self.K2_GetActorLocation`)) "AlwaysSpawn" "OverrideRootScale" null null)
  (`self.K2_DestroyActor`))

(event `self.ReceiveAnyDamage`
  (params (Damage :type "Float (single-precision)") (DamageType :type "DamageType Object Reference") (InstigatedBy :type "Controller Object Reference") (DamageCauser :type "Actor Object Reference"))
  (`|ExecutionSequence`
    (:`then_0`
      (`KismetSystemLibrary.Delay` 2.0)
      (`self.ServerSpawn`))
    (:`then_1`
      (`self.ServerActivateParticle`))))

(event `ServerSpawn`
  (`self.Multicast_Spawn`))

(event `ServerActivateParticle`
  (`self.MulticastParticle`))

(event `MulticastParticle`
  (`ActorComponent.Activate` (`self.ParticleSystem`) false))

(fn `UserConstructionScript`)