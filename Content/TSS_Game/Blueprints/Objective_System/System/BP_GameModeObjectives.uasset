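; Single-player objective game mode that tracks an ordered objective list and persists it, along with the player's weapons, in a BP_ObjectiveSave slot.
; BeginPlay loads progress, respawns saved weapons into the player's inventory and creates the W_Objectives HUD.
; A reverse loop leaves the first incomplete objective as current and on the HUD.
; Completing an objective replaces its entry with a completed copy, advances to the next and saves.
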(event `self.ReceiveBeginPlay`
  (bind _asbp_character_base_singleplayer (cast `/Game/Characters/BP_CharacterBase_Singleplayer` (`GameplayStatics.GetPlayerCharacter` 0))
    (:`then`
      (set `self.PlayerCast` _asbp_character_base_singleplayer))
    (:`CastFailed`
      _))
  (`self.LoadProgress`)
  (bind _returnvalue (`|CreateWidget` "/Game/TSS_Game/Blueprints/Objective_System/System/W_Objectives.W_Objectives_C"))
  (bind _output_get (set `self.Objective_HUD` _returnvalue))
  (`UserWidget.AddToViewport` _output_get 0)
  (`self.Start_Next_Objective`)
  (`self.SaveProgress`))

(event `Start_Next_Objective`
  ;[1 1 1] Setup Next Objective
  (bind (_arrayindex _arrayelement) (`/Engine/EditorBlueprintResources/StandardMacros.ReverseForEachLoop` (`self.Objectives`))
    (:`LoopBody`
      (bind (_objective_text_on_hud _iscompleted) (break `/Game/TSS_Game/Blueprints/Objective_System/System/S_ObjectiveData` _arrayelement))
      (if (not _iscompleted)
        (`/Game/TSS_Game/Blueprints/Objective_System/System/W_Objectives.Update_ObjectiveOnHUD` (`self.Objective_HUD`) _objective_text_on_hud)
        (set `self.CurrentObjectiveIndex` _arrayindex)))))

(event `Objective_Completed`
  (params (Objective_Index :type Integer))
  (bind _objectives (`self.Objectives`))
  ;[1 1 1] Objective Completed
  (for (_array_element _array_index) _objectives
    (if (== _array_index Objective_Index)
      (`KismetArrayLibrary.Array_Insert` _objectives (make `/Game/TSS_Game/Blueprints/Objective_System/System/S_ObjectiveData` (`.Objective_Text_On_HUD_8_348F398B4EB5EC548FD378B2B2B19C51` (break `/Game/TSS_Game/Blueprints/Objective_System/System/S_ObjectiveData` _array_element)) true) Objective_Index)
      (`KismetArrayLibrary.Array_Remove` _objectives (+ Objective_Index 1))))
  (`self.Start_Next_Objective`)
  (`self.SaveProgress`))

(fn `LoadProgress`
  (bind _playercast (`self.PlayerCast`))
  (bind _returnvalue (`GameplayStatics.DoesSaveGameExist` (`self.SaveSlotName`)))
  (if _returnvalue
    (bind _returnvalue_2 (`GameplayStatics.LoadGameFromSlot` (`self.SaveSlotName`)))
    (bind _asbp_objective_save (cast `/Game/TSS_Game/Blueprints/Objective_System/System/BP_ObjectiveSave` _returnvalue_2))
    (bind _output_get (set `self.SaveSlotProgress` _asbp_objective_save))
    (set `self.Objectives` (`/Game/TSS_Game/Blueprints/Objective_System/System/BP_ObjectiveSave.Objectives` _output_get))
    (`/Engine/EditorBlueprintResources/StandardMacros.IsValid` _playercast
      (:`Is Valid`
        (set `/Game/Characters/BP_CharacterBase.UseStartingWeapon` false _playercast)
        (`KismetArrayLibrary.Array_Clear` (`/Game/Characters/BP_CharacterBase.UT_Inventory` _playercast))
        (bind _savedweapons (`/Game/TSS_Game/Blueprints/Objective_System/System/BP_ObjectiveSave.SavedWeapons` _output_get))
        (if (> (`KismetArrayLibrary.Array_Length` _savedweapons) 0)
          (for _array_element _savedweapons
            (bind _returnvalue_3 (`|SpawnActorFromClass` _array_element (`KismetMathLibrary.MakeTransform` (0.0 0.0 0.0)) "AlwaysSpawn" "SelectDefaultAtRuntime" null null))
            (`/Game/TSS_Game/Blueprints/Weapons/Base/BP_WeaponBase.InteractWithWeapon` _returnvalue_3 (`self.PlayerCast`)))
          (else
            (`/Game/Characters/BP_CharacterBase.SpawnWeapon` _playercast (`/Game/Characters/BP_CharacterBase.DefaultWeaponClass` _playercast))))))
    (else
      (bind _returnvalue_4 (`GameplayStatics.CreateSaveGameObject` null))
      (bind _asbp_objective_save_2 (cast `/Game/TSS_Game/Blueprints/Objective_System/System/BP_ObjectiveSave` _returnvalue_4))
      (bind _output_get_2 (set `self.SaveSlotProgress` _asbp_objective_save_2))
      (set `self.Objectives` (`/Game/TSS_Game/Blueprints/Objective_System/System/BP_ObjectiveSave.Objectives` _output_get_2))
      (`GameplayStatics.SaveGameToSlot` _output_get_2 (`self.SaveSlotName`)))))

(fn `SaveProgress`
  (bind _playercast (`self.PlayerCast`))
  (bind _ut_inventory (`/Game/Characters/BP_CharacterBase.UT_Inventory` _playercast))
  (bind _returnvalue (`GameplayStatics.DoesSaveGameExist` (`self.SaveSlotName`)))
  (if _returnvalue
    (bind _returnvalue_2 (`GameplayStatics.LoadGameFromSlot` (`self.SaveSlotName`)))
    (bind _asbp_objective_save (cast `/Game/TSS_Game/Blueprints/Objective_System/System/BP_ObjectiveSave` _returnvalue_2))
    (bind _objectives (`/Game/TSS_Game/Blueprints/Objective_System/System/BP_ObjectiveSave.Objectives` _asbp_objective_save))
    (`KismetArrayLibrary.Array_Clear` _objectives)
    (for _array_element (`self.Objectives`)
      (`KismetArrayLibrary.Array_Add` _objectives _array_element))
    (`KismetArrayLibrary.Array_Clear` (`/Game/TSS_Game/Blueprints/Objective_System/System/BP_ObjectiveSave.SavedWeapons` _asbp_objective_save))
    (`/Engine/EditorBlueprintResources/StandardMacros.IsValid` _playercast
      (:`Is Valid`
        (if (> (`KismetArrayLibrary.Array_Length` _ut_inventory) 0)
          (for _array_element_2 _ut_inventory
            (`KismetArrayLibrary.Array_Add` (`/Game/TSS_Game/Blueprints/Objective_System/System/BP_ObjectiveSave.SavedWeapons` _asbp_objective_save) (`GameplayStatics.GetObjectClass` _array_element_2)))))
      (:`Is Not Valid`
        _))
    (`GameplayStatics.SaveGameToSlot` _asbp_objective_save (`self.SaveSlotName`))
    (else
      (bind _returnvalue_3 (`GameplayStatics.CreateSaveGameObject` "/Game/TSS_Game/Blueprints/Objective_System/System/BP_ObjectiveSave.BP_ObjectiveSave_C"))
      (bind _objectives_2 (`/Game/TSS_Game/Blueprints/Objective_System/System/BP_ObjectiveSave.Objectives` _returnvalue_3))
      (`KismetArrayLibrary.Array_Clear` _objectives_2)
      (for _array_element_3 (`self.Objectives`)
        (`KismetArrayLibrary.Array_Add` _objectives_2 _array_element_3))
      (`GameplayStatics.SaveGameToSlot` _returnvalue_3 (`self.SaveSlotName`)))))

(fn `UserConstructionScript`)