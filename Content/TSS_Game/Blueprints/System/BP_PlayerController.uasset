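; Player controller that handles character selection, HUD and session exit for online and local co-op play.
; On BeginPlay it takes the selected character from the game instance, with remote instances forwarding it via SetCharacter, which passes it to the game mode.
; It retries until a BP_CharacterBase pawn is possessed, then creates the HUD for local controller ID 0.
; Pause opens the disconnect widget; Kick removes the co-op player or disconnects online.
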(event `self.ReceiveBeginPlay`
  (bind _playercast (`self.PlayerCast`))
  (`|ExecutionSequence`
    (:`then_0`
      (if (`self.IsLocalPlayerController`)
        (bind _asbp_game_instance_with_settings (cast `/Game/TSS_Game/Blueprints/GameInstanceSettings/BP_GameInstanceWithSettings` (`GameplayStatics.GetGameInstance`)))
        (if (not (`/Game/TSS_Game/Blueprints/GameInstanceSettings/BP_GameInstanceWithSettings.IsLocalCoopGame` _asbp_game_instance_with_settings))
          (`EnhancedInputSubsystemInterface.AddMappingContext` (subsystem `EnhancedInputLocalPlayerSubsystem`) "/Game/TSS_Game/Blueprints/EnhancedInput/InputMapping_KeyboardMouse.InputMapping_KeyboardMouse" 0 (struct)))))
    (:`then_1`
      (bind _asbp_game_instance_with_settings_2 (cast `/Game/TSS_Game/Blueprints/GameInstanceSettings/BP_GameInstanceWithSettings` (`GameplayStatics.GetGameInstance`)))
      (bind _output_get (set `self.GameInstance_Cast` _asbp_game_instance_with_settings_2))
      (`/Engine/EditorBlueprintResources/ActorMacros.Switch Has Authority`
        (:`Authority`
          (bind _selectedcharacter (`/Game/TSS_Game/Blueprints/GameInstanceSettings/BP_GameInstanceWithSettings.SelectedCharacter` _output_get))
          (set `self.SelectedCharacter` _selectedcharacter))
        (:`Remote`
          (`self.Set_Character` _selectedcharacter)))
      (bind _asbp_character_base (cast `/Game/Characters/BP_CharacterBase` (`self.K2_GetPawn`) :!label _label)
        (:`then`
          (bind _output_get_2 (set `self.PlayerCast` _asbp_character_base))
          (set `/Game/Characters/BP_CharacterBase.OwningPlayerController` self _output_get_2)
          (`|ExecutionSequence`
            (:`then_0`
              (if (`self.IsLocalPlayerController`)
                (bind _asbp_game_instance_with_settings_3 (cast `/Game/TSS_Game/Blueprints/GameInstanceSettings/BP_GameInstanceWithSettings` (`GameplayStatics.GetGameInstance`)))
                (if (== (`/Game/TSS_Game/Blueprints/GameInstanceSettings/BP_GameInstanceWithSettings.LocalPlayers_Amount` _asbp_game_instance_with_settings_3) 0)
                  (cast `/Game/TSS_Game/Blueprints/Objective_System/System/BP_GameModeObjectives` (`GameplayStatics.GetGameMode`)))))
            (:`then_1`
              (`/Engine/EditorBlueprintResources/StandardMacros.IsValid` _playercast :!label _label_2
                (:`Is Valid`
                  (if (== (`GameplayStatics.GetPlayerControllerID` (`/Game/Characters/BP_CharacterBase.OwningPlayerController` _playercast)) 0)
                    (if (`self.IsLocalPlayerController`)
                      (`|ExecutionSequence`
                        (:`then_0`
                          (bind _returnvalue (`|CreateWidget` "/Game/TSS_Game/UI/W_PlayerHUD.W_PlayerHUD_C" null self))
                          (bind _output_get_3 (set `self.PlayerHUD` _returnvalue))
                          (`UserWidget.AddToViewport` _output_get_3 0)
                          (if (not (`/Game/TSS_Game/Blueprints/GameInstanceSettings/BP_GameInstanceWithSettings.IsLocalCoopGame` (`self.GameInstance_Cast`)))
                            (`Widget.SetVisibility` (`/Game/TSS_Game/UI/W_PlayerHUD.OtherPlayersInfo_VB` _output_get_3) "Hidden")))))))
                (:`Is Not Valid`
                  (`KismetSystemLibrary.Delay` 1.0)
                  (goto _label_2))))))
        (:`CastFailed`
          (`KismetSystemLibrary.Delay` 1.0)
          (`self.TryAgainCast`)
          (`KismetSystemLibrary.PrintString` "Hello"))))))

(event `SendSelectedCharToGameMode`
  (bind _asbp_game_mode_base (cast `/Game/TSS_Game/Blueprints/System/BP_GameModeBase` (`GameplayStatics.GetGameMode`)))
  (`/Game/TSS_Game/Blueprints/System/BP_GameModeBase.SetCharacter_Server` _asbp_game_mode_base self (`self.SelectedCharacter`)))

(event `Set_Character`
  (params (SelectedCharacter :type "/Game/Characters/BP_CharacterBase Class Reference"))
  (set `self.SelectedCharacter` SelectedCharacter)
  (`self.SendSelectedCharToGameMode`))

(event `TryAgainCast`
  (goto _label))

(event `EnhancedInput|/Game/TSS_Game/Blueprints/EnhancedInput/InputAction_Pause`
  (params (ActionValue :type Boolean) (ElapsedSeconds :type "Float (double-precision)") (TriggeredSeconds :type "Float (double-precision)") (InputAction :type "InputAction Object Reference" :default "/Game/TSS_Game/Blueprints/EnhancedInput/InputAction_Pause.InputAction_Pause"))
  (:`Triggered`
    (`/Engine/EditorBlueprintResources/StandardMacros.IsValid` (stale _returnvalue)
      (:`Is Valid`
        (`Widget.RemoveFromParent` (stale _returnvalue)))
      (:`Is Not Valid`
        _))
    (bind _returnvalue (`|CreateWidget` "/Game/TSS_Game/UI/W_Disconnect.W_Disconnect_C" null self))
    (`UserWidget.AddToViewport` _returnvalue 0)))

(event `Kick`
  (bind _gameinstance_cast (`self.GameInstance_Cast`))
  (if (`/Game/TSS_Game/Blueprints/GameInstanceSettings/BP_GameInstanceWithSettings.IsLocalCoopGame` _gameinstance_cast)
    (`GameplayStatics.RemovePlayer` self true)
    (set `/Game/TSS_Game/Blueprints/GameInstanceSettings/BP_GameInstanceWithSettings.LocalPlayers_Amount` (- (`/Game/TSS_Game/Blueprints/GameInstanceSettings/BP_GameInstanceWithSettings.LocalPlayers_Amount` _gameinstance_cast) 1) _gameinstance_cast)
    (else
      (`KismetSystemLibrary.ExecuteConsoleCommand` "disconnect" null))))

(fn `CompareControllerID`
  (params (ID :type Integer))
  (returns (True :type Boolean))
  (bind _playercast (`self.PlayerCast`))
  (`/Engine/EditorBlueprintResources/StandardMacros.IsValid` _playercast
    (:`Is Valid`
      (return (== (`GameplayStatics.GetPlayerControllerID` (`/Game/Characters/BP_CharacterBase.OwningPlayerController` _playercast)) ID)))))

(fn `UserConstructionScript`)