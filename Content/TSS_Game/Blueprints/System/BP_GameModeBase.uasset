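; Game mode that manages local split-screen and networked players, character spawning and kicking.
; On BeginPlay it creates local players from game instance settings, respawns tracked controllers' selected characters as a Blueprint ServerTravel workaround, and removes extra local players outside local co-op.
; PostLogin fills the controller list used for index-based kicking in non-co-op games.
; SetCharacter_Server replaces a controller's pawn with the chosen class at a random PlayerStart.
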(event `AddSplitScreenPlayer`
  (params (n :type Integer))
  ;[1 1 1] Split screen
  ;;[1 1 1] Create new local player for split screen
  (switch `int` n
    (:`1`
      (`GameplayStatics.CreatePlayer` -1))
    (:`2`
      (`GameplayStatics.CreatePlayer` -1)
      (`GameplayStatics.CreatePlayer` -1))
    (:`3`
      (`GameplayStatics.CreatePlayer` -1)
      (`GameplayStatics.CreatePlayer` -1)
      (`GameplayStatics.CreatePlayer` -1))))

(event `self.ReceiveBeginPlay`
  (`|ExecutionSequence`
    (:`then_0`
      ;[1 1 1] Split screen
      (bind _asbp_game_instance_with_settings (cast `/Game/TSS_Game/Blueprints/GameInstanceSettings/BP_GameInstanceWithSettings` (`GameplayStatics.GetGameInstance`)))
      (set `self.GameInstanceReference` _asbp_game_instance_with_settings)
      (bind _localplayers_amount (`/Game/TSS_Game/Blueprints/GameInstanceSettings/BP_GameInstanceWithSettings.LocalPlayers_Amount` _asbp_game_instance_with_settings))
      (if (not (== (`KismetArrayLibrary.Array_Length` (`GameStateBase.PlayerArray` (`GameplayStatics.GetGameState`))) (+ _localplayers_amount 1)))
        (`self.AddSplitScreenPlayer` _localplayers_amount)))
    (:`then_1`
      ;[1 1 1] ServerTravel workaround without making it in C++
      (for _array_element (`self.PlayerControllers`)
        (bind _returnvalue (`Controller.K2_GetPawn` _array_element))
        (`/Engine/EditorBlueprintResources/StandardMacros.IsValid` _returnvalue
          (:`Is Valid`
            (`self.K2_DestroyActor` _returnvalue)
            (bind _outactors (`GameplayStatics.GetAllActorsOfClass` "/Script/Engine.PlayerStart"))
            (`KismetSystemLibrary.Delay` 0.2)
            (bind _asbp_player_controller (cast `/Game/TSS_Game/Blueprints/System/BP_PlayerController` _array_element :!pure true))
            (bind _returnvalue_2 (`|SpawnActorFromClass` (`/Game/TSS_Game/Blueprints/System/BP_PlayerController.SelectedCharacter` _asbp_player_controller) (`self.GetTransform` (`|GetArrayItem` _outactors)) "AlwaysSpawn" "SelectDefaultAtRuntime" null null))
            (`Controller.Possess` _asbp_player_controller _returnvalue_2)
            (`/Game/TSS_Game/Blueprints/System/BP_PlayerController.TryAgainCast` _asbp_player_controller)
            (`self.RestartPlayer` _asbp_player_controller)))))
    (:`then_2`
      (bind _asbp_game_instance_with_settings_2 (cast `/Game/TSS_Game/Blueprints/GameInstanceSettings/BP_GameInstanceWithSettings` (`GameplayStatics.GetGameInstance`)))
      (if (not (`/Game/TSS_Game/Blueprints/GameInstanceSettings/BP_GameInstanceWithSettings.IsLocalCoopGame` _asbp_game_instance_with_settings_2))
        (for _array_element_2 (`GameStateBase.PlayerArray` (`GameplayStatics.GetGameState`))
          (bind _asbp_player_state (cast `/Game/TSS_Game/Blueprints/System/BP_PlayerState` _array_element_2))
          (bind _asplayer_controller (cast `PlayerController` (`self.GetOwner` _asbp_player_state)))
          (if (not (== (`GameplayStatics.GetPlayerControllerID` _asplayer_controller) 0))
            (`GameplayStatics.RemovePlayer` _asplayer_controller true)))))))

(event `self.K2_PostLogin`
  (params (NewPlayer :type "PlayerController Object Reference"))
  (bind _asbp_game_instance_with_settings (cast `/Game/TSS_Game/Blueprints/GameInstanceSettings/BP_GameInstanceWithSettings` (`GameplayStatics.GetGameInstance`)))
  (if (not (`/Game/TSS_Game/Blueprints/GameInstanceSettings/BP_GameInstanceWithSettings.IsLocalCoopGame` _asbp_game_instance_with_settings))
    (if (not (== (`GameplayStatics.GetPlayerControllerID` NewPlayer) 0))
      (`GameplayStatics.RemovePlayer` NewPlayer true))
    (`/Engine/EditorBlueprintResources/StandardMacros.IsValid` NewPlayer
      (:`Is Valid`
        (bind _returnvalue (`KismetArrayLibrary.Array_Add` (`self.PlayerControllers`) NewPlayer))))))

(event `KickPlayer`
  (params (PlayerID :type Integer))
  ;[1 1 1] Kicks a player (Press P/ESC to open the menu)
  (for (_array_element _array_index) (`self.PlayerControllers`)
    (if (== _array_index PlayerID)
      (`/Engine/EditorBlueprintResources/StandardMacros.IsValid` _array_element
        (:`Is Valid`
          (bind _asbp_player_controller (cast `/Game/TSS_Game/Blueprints/System/BP_PlayerController` _array_element))
          (`/Game/TSS_Game/Blueprints/System/BP_PlayerController.Kick` _asbp_player_controller))))))

(event `SetCharacter_Server`
  (params (ControllerReference :type "/Game/TSS_Game/Blueprints/System/BP_PlayerController Object Reference") (CharacterClass :type "Character Class Reference"))
  (bind _returnvalue (`Controller.K2_GetPawn` ControllerReference))
  ;[1 1 1] Spawn selected character
  (`/Engine/EditorBlueprintResources/StandardMacros.IsValid` _returnvalue
    (:`Is Valid`
      (`self.K2_DestroyActor` _returnvalue))
    (:`Is Not Valid`
      _))
  (bind _outactors (`GameplayStatics.GetAllActorsOfClass` "/Script/Engine.PlayerStart"))
  (bind _returnvalue_2 (`|SpawnActorFromClass` CharacterClass (`self.GetTransform` (`|GetArrayItem` _outactors (`KismetMathLibrary.RandomIntegerInRange` 0 (- (`KismetArrayLibrary.Array_Length` _outactors) 1)))) "AlwaysSpawn" "SelectDefaultAtRuntime" ControllerReference null))
  (`Controller.Possess` ControllerReference _returnvalue_2)
  (`/Game/TSS_Game/Blueprints/System/BP_PlayerController.TryAgainCast` ControllerReference)
  (`/Engine/EditorBlueprintResources/StandardMacros.IsValid` _returnvalue_2
    (:`Is Valid`
      _)
    (:`Is Not Valid`
      _))
  (`self.RestartPlayer` ControllerReference))

(fn `UserConstructionScript`)