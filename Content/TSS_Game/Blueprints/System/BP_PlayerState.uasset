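; BP_PlayerState is a player state that tracks a score and player number.
; On BeginPlay or Start, it caches player character 0 as BP_CharacterBase and sets PlayerNumber to the current PlayerArray length.
; InteractwithWeapon calls AddScore, which increments PlayerScore by one.
; The free-for-all score HUD creation is disconnected, and the local-controller check leads to no action.
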(event `Start`
  (bind _asbp_character_base (cast `/Game/Characters/BP_CharacterBase` (`GameplayStatics.GetPlayerCharacter` 0) :!label _label))
  (set `self.PlayerCast` _asbp_character_base)
  (set `self.PlayerNumber` (`KismetArrayLibrary.Array_Length` (`GameState.PlayerArray` (`GameplayStatics.GetGameState`))))
  (if (`Controller.IsLocalPlayerController` (`GameplayStatics.GetPlayerController` 0))
    _))

(event `self.ReceiveBeginPlay`
  (goto _label))

(event `/Game/TSS_Game/Blueprints/System/BPI_Interactive.InteractWithWeapon`
  (params (CharacterReference :type "/Game/Characters/BP_CharacterBase Object Reference"))
  (`self.AddScore`))

(fn `AddScore`
  (set `self.PlayerScore` (+ (`self.PlayerScore`) 1)))

(fn `UserConstructionScript`)