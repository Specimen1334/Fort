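; Base ammo pickup whose child classes set the ammo name shown on its floating text, held at a fixed world rotation each tick.
; When an overlapping BP_CharacterBase has an equipped weapon, it searches UTInventory for an exact WeaponClass match.
; If that weapon's reserve is not at max, it adds one AmmoMax amount clamped to the limit, plays a sound and destroys itself.
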(event `self.ReceiveBeginPlay`
  (`TextRenderComponent.K2_SetText` (`self.AmmoNameTXT`) (`self.AmmoName`)) ; This gets set from ammo child classes
)

(event `self.ReceiveTick`
  (params (DeltaSeconds :type "Float (single-precision)"))
  (`SceneComponent.K2_SetWorldRotation` (`self.AmmoNameTXT`) (struct :`Pitch` 45.0 :`Yaw` 180.0) false false) ; Rotates the text to face the camera
)

(event `self.ReceiveActorBeginOverlap`
  (params (OtherActor :type "Actor Object Reference"))
  ;[1 1 1] Checks for ammo and the weapon child class that it's for, if player has the weapon and ammo isn't at max, if true: add ammo, play sound, destroy pickup
  (bind _asbp_character_base (cast `/Game/Characters/BP_CharacterBase` OtherActor))
  (`/Engine/EditorBlueprintResources/StandardMacros.IsValid` (`/Game/Characters/BP_CharacterBase.EquippedWeapon` _asbp_character_base)
    (:`Is Valid`
      (for _array_element (`/Game/Characters/BP_CharacterBase.UT_Inventory` _asbp_character_base)
        (if (== (`self.WeaponClass`) (`GameplayStatics.GetObjectClass` _array_element))
          (if (not (== (`/Game/TSS_Game/Blueprints/Weapons/Base/BP_WeaponBase.AmmoInReserveMax` _array_element) (`/Game/TSS_Game/Blueprints/Weapons/Base/BP_WeaponBase.AmmoInReserve` _array_element)))
            (set `/Game/TSS_Game/Blueprints/Weapons/Base/BP_WeaponBase.AmmoInReserve` (`KismetMathLibrary.Clamp` (+ (`/Game/TSS_Game/Blueprints/Weapons/Base/BP_WeaponBase.AmmoInReserve` _array_element) (`/Game/TSS_Game/Blueprints/Weapons/Base/BP_WeaponBase.AmmoMax` _array_element)) 0 (`/Game/TSS_Game/Blueprints/Weapons/Base/BP_WeaponBase.AmmoInReserveMax` _array_element)) _array_element)
            (`GameplayStatics.PlaySoundAtLocation` "/Game/TSS_Game/SFX/Pickup/SFX_Coin_Cue.SFX_Coin_Cue" (`self.K2_GetActorLocation`) (struct) 1.0 1.0 0.0 null null null null)
            (`self.K2_DestroyActor`)))))))

(fn `UserConstructionScript`)